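; GA_Punch is a Gameplay Ability for a punch attack that commits, then plays a right hook montage.
; A one-shot wait for the hit gameplay event applies GE_PunchEffect to the event's target data.
; Montage completion ends the ability, blend out or interruption cancels it, and OnEndAbility cleans up async tasks.
; The random punch choice is an empty placeholder, and the uppercut, equipped and montage-task variants are disconnected.
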(event `self.K2_ActivateAbility`
  (bind (_returnvalue_owneractor _returnvalue_avataractor _returnvalue_playercontroller _returnvalue_abilitysystemcomponent _returnvalue_skeletalmeshcomponent) (break `GameplayAbilityActorInfo` (`self.GetActorInfo`)))
  ;[1 1 1] Start and Commit Ability
  (bind _returnvalue (`self.K2_CommitAbility`))
  (if _returnvalue
    ;[1 1 1] Unequipped - Random Swap Punch Type
    (if (`KismetMathLibrary.RandomBool`)
      _
      (else
        _))
    (`|PlayMontage` _returnvalue_skeletalmeshcomponent "/Game/Characters/Knight/Animations/AM_RightHook.AM_RightHook"
      (:`then`
        (bind (_asynctaskproxy _payload) (`AbilityTask_WaitGameplayEvent.WaitGameplayEvent` (struct :`TagName` "Event.InitialAbility.Hit") null true)
          (:`then`
            (set `self.Async Wait Gameplay Task` _asynctaskproxy))
          (:`EventReceived`
            (`KismetSystemLibrary.PrintString` "Hit received!")
            (`self.BP_ApplyGameplayEffectToTarget` (`.TargetData` (break `GameplayEventData` _payload)) "/Game/Abilities/Punch/GE_PunchEffect.GE_PunchEffect_C"))))
      (:`OnCompleted`
        (`self.K2_EndAbility`))
      (:`OnBlendOut`
        (`self.K2_CancelAbility` :!label _label))
      (:`OnInterrupted`
        (goto _label)))
    (else
      (`self.K2_CancelAbility`))))

(event `self.K2_OnEndAbility`
  (params (bWasCancelled :type Boolean))
  (bind _async_wait_gameplay_task (`self.Async Wait Gameplay Task`))
  (bind _async_montage_task (`self.Async Montage Task`))
  ;[1 1 1] End Ability
  (`/Engine/EditorBlueprintResources/StandardMacros.IsValid` _async_wait_gameplay_task
    (:`Is Valid`
      (`GameplayTask.EndTask` _async_wait_gameplay_task))
    (:`Is Not Valid`
      _))
  (`/Engine/EditorBlueprintResources/StandardMacros.IsValid` _async_montage_task
    (:`Is Valid`
      (`GameplayTask.EndTask` _async_montage_task))))