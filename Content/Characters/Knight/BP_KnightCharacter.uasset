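; Knight character Blueprint that handles hit detection for its initial Gameplay Ability.
; HandleNotifyInitialAbility runs a sphere overlap for pawns at the RightHand socket, ignoring itself.
; The first pawn found is packed as target and target data into an Event.InitialAbility.Hit gameplay event sent to the instigator.
; Only that single target is reported per call, and the construction script is empty.
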(event `self.HandleNotifyInitialAbility`
  (bind _returnvalue (`self.GetInstigator`))
  ;[1 1 1] Initial Ability Event
  (bind _outactors (`KismetSystemLibrary.SphereOverlapActors` (`SceneComponent.GetSocketLocation` (`self.Mesh`) "RightHand") 50.0 (`|MakeArray` "ObjectTypeQuery3" :!type "EObjectTypeQuery Enum") null (`|MakeArray` self :!type "Actor Object Reference"))) ; Could Loop i want more actors
  (if (`KismetArrayLibrary.Array_IsValidIndex` _outactors)
    (bind _output (`|GetArrayItem` _outactors))
    (`AbilitySystemBlueprintLibrary.SendGameplayEventToActor` _returnvalue (struct :`TagName` "Event.InitialAbility.Hit") (make `GameplayEventData` (struct) _returnvalue _output null null (struct) (struct) (struct) 0.0 (`AbilitySystemBlueprintLibrary.AbilityTargetDataFromActor` _output)))))

(fn `UserConstructionScript`)