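; BP_LootDummy is a test enemy that stands in for loot dropping on death.
; OnDeath loops over its Inventory items and prints each display name, without spawning any pickups.
; The ragdoll, pawn-collision ignore and three-second delayed destroy sit inside that loop, so they run only when the inventory holds items.
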(event `self.On_Death`
  ;[1 1 1] On Death Spawn Loot
  (`KismetSystemLibrary.PrintString` "Drop ze loot!")
  (for _array_element (`InventoryComponent.Items` (`self.Inventory`))
    (`KismetSystemLibrary.PrintString` (`KismetSystemLibrary.GetDisplayName` _array_element))
    ;[1 1 1] Die and Despawn
    (`PrimitiveComponent.SetCollisionResponseToChannel` (`self.Mesh`) "ECC_Pawn" "ECR_Ignore")
    (`PrimitiveComponent.SetSimulatePhysics` (`self.Mesh`) true)
    (`KismetSystemLibrary.Delay` 3.0)
    (`self.K2_DestroyActor`))
  (`KismetSystemLibrary.PrintString` "Items Done"))

(fn `UserConstructionScript`)